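; VideoScreen is an AugmentedUnreality Blueprint that connects a Screen to a video driver.
; Initialize constructs a driver object from the configurable VideoDriverClass, initializes it and passes it to Screen.
; BeginPlay runs Initialize only if no valid driver exists, so earlier initialization is respected.
; EndPlay deactivates the Screen and shuts down the driver.
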(event EventBeginPlay
  ;[1 1 1] Initialize (create driver) if not initialized earlier
  (Utilities|IsValid (Variables|Default|GetDriverInstance)
    (:Is%20Not%20Valid
      (CallFunction|Initialize))))

(event EventEndPlay
  (params (EndPlayReason :type EEndPlayReason%20Enum :default "Destroyed"))
  (Components|Activation|Deactivate (Variables|Default|GetScreen))
  (Class|AURDriver|Shutdown (Variables|Default|GetDriverInstance)))

(fn ConstructionScript)

(fn Initialize
  (bind _returnvalue (Game|ConstructObjectfromClass (Variables|Default|GetVideoDriverClass) self))
  (bind _output_get (Variables|Default|SetDriverInstance _returnvalue))
  (Class|AURDriver|Initialize _output_get)
  (Class|AURVideoScreenBase|Initialize (Variables|Default|GetScreen) _output_get))