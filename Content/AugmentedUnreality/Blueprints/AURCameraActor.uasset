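; AURCameraActor is an augmented reality camera actor whose transform follows the orientation reported by a driver.
; On BeginPlay it creates a driver from DriverClass, initializes it, hands it to the Screen component, and sets the camera's field of view from the driver's camera parameters.
; Each tick it applies the driver's orientation as the actor transform.
; On EndPlay it deactivates the screen and shuts the driver down.
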(event EventBeginPlay
  (bind _returnvalue (Game|ConstructObjectfromClass (Variables|AugmentedReality|GetDriverClass) self))
  (bind _output_get (Variables|AugmentedReality|SetDriverInstance _returnvalue))
  (Class|AURDriver|Initialize _output_get)
  (Class|AURVideoScreenBase|Initialize (Variables|Default|GetScreen) _output_get)
  (bind _field_of_view_angle (Class|AURDriver|GetCameraParameters _output_get))
  (Variables|/Script/Engine.CameraComponent|SetFieldOfView (Variables|CameraActor|GetCameraComponent) _field_of_view_angle))

(event EventTick
  (params (DeltaSeconds :type Float%20%28single-precision%29))
  (bind _returnvalue (Class|AURDriver|GetOrientation (Variables|AugmentedReality|GetDriverInstance)))
  (Transformation|SetActorTransform _returnvalue))

(event EventEndPlay
  (params (EndPlayReason :type EEndPlayReason%20Enum :default "Destroyed"))
  (Components|Activation|Deactivate (Variables|Default|GetScreen))
  (Class|AURDriver|Shutdown (Variables|AugmentedReality|GetDriverInstance)))

(fn ConstructionScript)