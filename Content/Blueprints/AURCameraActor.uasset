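; Augmented reality camera actor that drives an AUR video/tracking driver and moves with the viewpoint it reports.
; A one-time Initialize reuses or creates the driver, optionally adds a diagnostic UI for OpenCV drivers, and opens the default video source.
; Driver callbacks update the actor transform and match camera FOV and screen size to the video.
; Marker board spawning is disconnected, and a smoothed static-camera pose handler exists separately.
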(event Custom|Initialize
  (params (OwningController :type Player%20Controller%20Object%20Reference))
  (bind _driverinstance (Variables|AugmentedReality|GetDriverInstance))
  (Utilities|FlowControl|DoOnce false
    (:Completed
      (AugmentedReality|InitializeDriver)
      (CallFunction|InitializeUI OwningController)
      (AugmentedReality|InitializeMarkerBoard)
      (AugmentedReality|InitializeScreen)
      ;[1 1 1] Listen for changes in FOV to update camera
      (EventDispatchers|BindEventtoOnVideoPropertiesChange _driverinstance (EventDispatchers|CreateEvent :!event VideoPropertiesChanged))
      (CallFunction|VideoPropertiesChanged _driverinstance)
      ;[1 1 1] Start video stream
      (Class|AURDriver|OpenVideoSourceDefault _driverinstance)
      (EventDispatchers|BindEventtoOnViewpointTransformUpdate _driverinstance (delegate Custom|OnViewpointUpdate))
      ;[1 1 1] Align the viewpoint initially so that main marker is not needed to position tracked objects
      (Transformation|SetActorTransform (Class|AURDriver|GetCurrentViewportTransform (Variables|AugmentedReality|GetDriverInstance))))))

(event Custom|OnViewpointUpdate
  (params (Driver :type AUR%20Driver%20Object%20Reference) (ViewportTransform :type Transform))
  (Transformation|SetActorTransform ViewportTransform))

(event EventBeginPlay
  (bind _returnvalue (Class|CameraActor|GetAutoActivatePlayerIndex))
  (bind _returnvalue_2 (Game|GetPlayerController _returnvalue))
  (if (>= _returnvalue 0)
    (Utilities|IsValid _returnvalue_2
      (:Is%20Valid
        (CallFunction|Initialize _returnvalue_2)))))

(event EventTick
  (params (DeltaSeconds :type Float%20%28single-precision%29))
  (Class|AURDriver|Tick (Variables|AugmentedReality|GetDriverInstance)))

(event EventEndPlay
  (params (EndPlayReason :type EEndPlayReason%20Enum :default "Destroyed"))
  (Class|AURDriver|Shutdown (Variables|AugmentedReality|GetDriverInstance)))

(fn ConstructionScript)

(fn SetFOV
  (params (FOV :type Float%20%28single-precision%29))
  (if (!= FOV (Variables|AugmentedReality|GetCurrentFOV))
    (bind _output_get (Variables|AugmentedReality|SetCurrentFOV FOV))
    (Camera|SetFieldOfView (Variables|CameraActor|GetCameraComponent) _output_get)
    (Class|AURVideoScreenBackground|SetSizeforFOV (Variables|Default|GetScreen) _output_get)))

(fn InitializeScreen
  (AugmentedReality|SetFOV (Variables|AugmentedReality|GetDefaultFOV)))

(fn InitializeMarkerBoard)

(fn SetBoardActorVisibility
  (params (Visible :type Boolean))
  (bind _output_get (Variables|AugmentedReality|SetBoardActorVisible Visible))
  (for _array_element (Variables|AugmentedReality|GetBoards)
    _))

(fn VideoPropertiesChanged
  (params (Driver :type AUR%20Driver%20Object%20Reference))
  (if (Class|AURDriver|IsConnected Driver)
    (AugmentedReality|SetFOV (.X (Math|Vector2D|BreakVector2D (Class|AURDriver|GetFieldOfView Driver))))))

(fn SetStaticCameraModeActive
  (params (Active :type Boolean))
  (Variables|ARStaticCamera|SetStaticCameraModeActive Active))

(fn OnTrackingUpdate
  (params (NewPose :type Transform))
  (if (Variables|ARStaticCamera|GetStaticCameraModeActive)
    (Transformation|SetActorTransform (Math|Transform|Lerp(Transform) (Transformation|GetActorTransform) NewPose (- 1.0 (Variables|ARStaticCamera|GetStaticCameraSmoothing))))
    (else
      (Transformation|SetActorTransform NewPose))))

(fn InitializeDriver
  ;[1 1 1] Already initialized
  (Utilities|IsValid (Variables|AugmentedReality|GetDriverInstance)
    (:Is%20Not%20Valid
      ;[1 1 1] Driver created by someone else
      (bind _returnvalue (Class|AURDriver|GetCurrentDriver))
      (Utilities|IsValid _returnvalue
        (:Is%20Valid
          (Variables|AugmentedReality|SetDriverInstance _returnvalue))
        (:Is%20Not%20Valid
          ;[1 1 1] Create new driver
          (bind _returnvalue_2 (Game|ConstructObjectfromClass (Variables|AugmentedReality|GetDriverClass) self))
          (bind _output_get (Variables|AugmentedReality|SetDriverInstance _returnvalue_2))
          (Class|AURDriver|Initialize _output_get self))))))

(fn InitializeUI
  (params (OwningController :type Player%20Controller%20Object%20Reference))
  (if (Variables|AugmentedReality|GetCreateUI)
    (bind _asaurdriver_open_cv (Utilities|Casting|CastToAURDriverOpenCV (Variables|AugmentedReality|GetDriverInstance)))
    (bind _returnvalue (UserInterface|CreateWidget "/AugmentedUnreality/Blueprints/UI/AURUIDiagnosticView.AURUIDiagnosticView_C" OwningController _asaurdriver_open_cv false))
    (UserInterface|Viewport|AddtoViewport _returnvalue 0)))