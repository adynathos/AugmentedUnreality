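; ShadowPlane is an actor whose FloorScreen component displays a driver's output texture, presumably as a shadow surface.
; UseDriver stores the given driver and subscribes to its camera-parameter change event.
; On each change, a valid output texture is written to the VideoTexture parameter of a dynamic material.
; That material instance is created lazily on FloorScreen's first slot and cached for reuse.
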(event Custom|UseDriver
  (params (NewDriver :type AUR%20Driver%20Object%20Reference))
  (bind _output_get (Variables|Default|SetDriver NewDriver))
  (Utilities|IsValid _output_get
    (:Is%20Valid
      (EventDispatchers|BindEventtoOnCameraParametersChange _output_get (delegate Custom|OnCameraPropertiesChanged)))))

(event Custom|OnCameraPropertiesChanged
  (params (Driver :type AUR%20Driver%20Object%20Reference))
  (bind _returnvalue (Class|AURDriver|GetOutputTexture Driver))
  (Utilities|IsValid _returnvalue
    (:Is%20Valid
      (CallFunction|SetDynamicTexture _returnvalue))))

(event EventBeginPlay)

(event Collision|EventActorBeginOverlap
  (params (OtherActor :type Actor%20Object%20Reference)))

(event EventTick
  (params (DeltaSeconds :type Float%20%28single-precision%29)))

(fn ConstructionScript)

(fn GetDynamicMaterial
  (bind _floorscreen (Variables|Default|GetFloorScreen))
  (Utilities|IsValid (Variables|Default|GetDynamicMaterial)
    (:Is%20Valid
      _)
    (:Is%20Not%20Valid
      (bind _returnvalue (Rendering|Material|CreateDynamicMaterialInstance _floorscreen 0 0 :!class /Script/Engine.PrimitiveComponent))
      (Rendering|Material|SetMaterial _floorscreen 0 _returnvalue)
      (Variables|Default|SetDynamicMaterial _returnvalue)))
  (return (Variables|Default|GetDynamicMaterial)))

(fn SetDynamicTexture
  (params (NewTexture :type Texture%202D%20Object%20Reference))
  (bind _materialinstance (CallFunction|GetDynamicMaterial))
  (Rendering|Material|SetTextureParameterValue _materialinstance "VideoTexture" NewTexture))