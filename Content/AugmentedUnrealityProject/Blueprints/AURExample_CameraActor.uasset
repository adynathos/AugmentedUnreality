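; Example camera actor for the Augmented Unreality project that links its AUR driver instance to an owning player controller.
; SetOwningController stores the controller and calls its OnAURDriverActivated if the driver instance is already valid.
; BeginPlay makes the same notification, passing itself as the camera actor, if an owner is already set, covering either initialization order.
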(event EventBeginPlay
  (bind _owningplayer (Variables|Default|GetOwningPlayer))
  (|CallParentFunction)
  (Utilities|IsValid _owningplayer
    (:Is%20Valid
      (Default|OnAURDriverActivated _owningplayer (Variables|Default|GetDriverInstance) self))))

(event EventTick
  (params (DeltaSeconds :type Float%20%28single-precision%29))
  (|CallParentFunction 0.0))

(fn ConstructionScript
  (|CallParentFunction))

(fn SetOwningController
  (params (PC :type AUR%20Example%20Player%20Controller%20Object%20Reference))
  (bind _driverinstance (Variables|Default|GetDriverInstance))
  (bind _output_get (Variables|Default|SetOwningPlayer PC))
  (Utilities|IsValid _driverinstance
    (:Is%20Valid
      (Default|OnAURDriverActivated _output_get _driverinstance))))