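; Player controller for the AugmentedUnrealityProject example that links the AR camera actor and AR driver to a status UI.
; On BeginPlay it casts the AURCamera child actor to the example camera actor and registers itself as owning controller.
; When a driver activates, it stores the instance, creates the status view widget once, adds it to the viewport, and passes it the driver and camera actor.
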(event EventBeginPlay
  (bind _asaurexample_camera_actor (Utilities|Casting|CastToAURExample_CameraActor (Variables|/Script/Engine.ChildActorComponent|GetChildActor (Variables|Default|GetAURCamera))))
  (Default|SetOwningController _asaurexample_camera_actor self))

(event EventTick
  (params (DeltaSeconds :type Float%20%28single-precision%29)))

(fn ConstructionScript)

(fn OnAURDriverActivated
  (params (DriverInstance :type AUR%20Driver%20Object%20Reference) (CamActor :type AUR%20Camera%20Actor%20Object%20Reference))
  (Variables|AugmentedReality|SetAURDriverInstance DriverInstance)
  (Utilities|IsValid (Variables|AugmentedReality|GetAURStatusView)
    (:Is%20Valid
      _)
    (:Is%20Not%20Valid
      (bind _returnvalue (UserInterface|CreateWidget "/Game/AugmentedUnrealityProject/Blueprints/UI/AUR_StatusView.AUR_StatusView_C" self))
      (bind _output_get (Variables|AugmentedReality|SetAURStatusView _returnvalue))
      (UserInterface|Viewport|AddtoViewport _output_get 0)))
  (Default|OnDriverActivated (Variables|AugmentedReality|GetAURStatusView) (Variables|AugmentedReality|GetAURDriverInstance) CamActor))