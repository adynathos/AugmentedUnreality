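; Example AR player controller that sets up the AUR camera and its diagnostic UI when play begins.
; It spawns an AURCameraActor at a fixed transform with the configured camera driver class, then initializes it.
; If the driver instance is valid, it creates the diagnostic widget once, adds it to the viewport and binds it to that driver.
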(event EventBeginPlay
  (bind _returnvalue (Game|SpawnActorfromClass "/Game/AugmentedUnreality/Blueprints/AURCameraActor.AURCameraActor_C" (Math|Transform|MakeTransform "0.000000, 0,500.000000" "90.000000, 0, 0") "Undefined" self (Variables|AugmentedReality|GetCameraDriverClass) 0))
  (bind _output_get (Variables|AugmentedReality|SetCameraActor _returnvalue))
  (Default|Initialize _output_get)
  (Utilities|IsValid (Variables|/Game/AugmentedUnreality/Blueprints/AURCameraActor.AURCameraActor_C|GetDriverInstance _output_get)
    (:Is%20Valid
      (CallFunction|CreateAURDiagnosticUI (Variables|/Game/AugmentedUnreality/Blueprints/AURCameraActor.AURCameraActor_C|GetDriverInstance _output_get)))))

(event EventTick
  (params (DeltaSeconds :type Float%20%28single-precision%29)))

(fn ConstructionScript)

(fn CreateAURDiagnosticUI
  (params (DriverInstance :type AUR%20Driver%20Object%20Reference))
  (Variables|AugmentedReality|SetAURDriverInstance DriverInstance)
  (Utilities|IsValid (Variables|AugmentedReality|GetAURStatusView)
    (:Is%20Valid
      _)
    (:Is%20Not%20Valid
      (bind _returnvalue (UserInterface|CreateWidget "/Game/AugmentedUnreality/Blueprints/CameraDiagnosticView.CameraDiagnosticView_C" self))
      (bind _output_get (Variables|AugmentedReality|SetAURStatusView _returnvalue))
      (UserInterface|Viewport|AddtoViewport _output_get 0)))
  (Default|SetDriver (Variables|AugmentedReality|GetAURStatusView) (Variables|AugmentedReality|GetAURDriverInstance)))