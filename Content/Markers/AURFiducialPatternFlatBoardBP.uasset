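; Fiducial marker flat board actor, a visual stand-in for an OpenCV tracking pattern identified by its starting marker ID.
; The construction script scales the board mesh from board dimensions and square size, swapping width and height to match OpenCV's axes.
; It also labels the board "CHA" plus the starting ID.
; BeginPlay only prints the root component's attach parent name and class for debugging.
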(event EventBeginPlay
  (bind _defaultsceneroot (Variables|Default|GetDefaultSceneRoot))
  (bind _returnvalue (Transformation|GetAttachParent _defaultsceneroot))
  (Development|PrintString (Utilities|String|Append "Board's parent:" (Utilities|GetDisplayName _returnvalue) " cls = " (Utilities|GetClassDisplayName (Utilities|GetClass _returnvalue)))))

(event Collision|EventActorBeginOverlap
  (params (OtherActor :type Actor%20Object%20Reference)))

(event EventTick
  (params (DeltaSeconds :type Float%20%28single-precision%29)))

(fn ConstructionScript
  (Transformation|SetRelativeScale3D (Variables|Default|GetBoardMesh) (* (Math|Vector|MakeVector (Math|Conversions|ToFloat(Integer) (Variables|Default|GetBoardHeight)) (Math|Conversions|ToFloat(Integer) (Variables|Default|GetBoardWidth)) 1.0) (/ (Variables|Default|GetSquareSize) 1e+01)))
  (Rendering|Components|TextRender|SetText (Variables|Default|GetBoardName) (Utilities|Text|FormatText "CHA 
{id}" (Variables|Default|GetMarkerIdSequenceStart))))